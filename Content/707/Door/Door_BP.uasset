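; Door Blueprint that animates two door leaves, RightMoon and LeftMoon, automatically when play begins.
; BeginPlay plays the TL_DoorMove timeline, whose two tracks set each leaf's relative yaw on every update while keeping pitch and roll.
; A separate custom event plays a second timeline with nothing connected to its outputs; overlap and Tick events are empty.
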(event `커스텀이벤트_0`
  (`Timeline|타임라인_0`))

(event `self.ReceiveBeginPlay`
  (bind _leftmoon (`self.LeftMoon`))
  (bind (_direction _leftmoon_2 _rightmoon) (`Timeline|TL_DoorMove`)
    (:`Update`
      (`SceneComponent.K2_SetRelativeRotation` (`self.RightMoon`) (`KismetMathLibrary.MakeRotator` (.roll (`SceneComponent.RelativeRotation` (`self.RightMoon`))) (.pitch (`SceneComponent.RelativeRotation` (`self.RightMoon`))) _rightmoon) false false)
      (`SceneComponent.K2_SetRelativeRotation` _leftmoon (`KismetMathLibrary.MakeRotator` (.roll (`SceneComponent.RelativeRotation` _leftmoon)) (.pitch (`SceneComponent.RelativeRotation` _leftmoon)) _leftmoon_2) false false))))

(fn `UserConstructionScript`)